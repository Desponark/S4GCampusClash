(event `self.ReceiveBeginPlay`
  (bind _levelnames (`self.levelNames`))
  (`/Engine/EditorBlueprintResources/ActorMacros.Switch Has Authority`
    (:`Authority`
      (`self.Initialize`)
      (bind _output_get (set `self.loadedLevelName` (`|GetArrayItem` _levelnames (`KismetMathLibrary.RandomInteger` (`KismetArrayLibrary.Array_Length` _levelnames)))))
      (`GameplayStatics.LoadStreamLevel` (`KismetStringLibrary.Conv_StringToName` _output_get) true true)
      (`self.InitNewLevel`))))

(event `PlayerJoinEvent`
  (params (player :type "/Game/StarterContent/ThirdPerson/Blueprints/BP_ThirdPersonCharacter Object Reference"))
  (bind _asbp_player_controller (cast `/Game/CampusClash/Core/Controllers/BP_PlayerController` (`Pawn.GetController` player)))
  (`self.PlayerJoin` _asbp_player_controller))

(event `HandleCountdown`
  (for _array_element (`self.FYWCharacters`)
    (`/Game/CampusClash/Placeables/FindYourWay/BP_FYW_Character.ClientEvent StartCountdown` _array_element)
    (`/Game/CampusClash/Placeables/FindYourWay/BP_FYW_Character.ClientEvent PlaySound` _array_element (`BlueprintMapLibrary.Map_Find` (`self.soundList`) "Countdown")))
  (`KismetSystemLibrary.Delay` 1.0)
  (if (`self.isGameOngoing`)
    (for _array_element_2 (`self.FYWCharacters`)
      (`/Game/CampusClash/Placeables/FindYourWay/BP_FYW_Character.ClientEvent UpdateCountdown` _array_element_2 "2")
      (`/Game/CampusClash/Placeables/FindYourWay/BP_FYW_Character.ClientEvent PlaySound` _array_element_2 (`BlueprintMapLibrary.Map_Find` (`self.soundList`) "Countdown")))
    (`KismetSystemLibrary.Delay` 1.0)
    (if (`self.isGameOngoing`)
      (for _array_element_3 (`self.FYWCharacters`)
        (`/Game/CampusClash/Placeables/FindYourWay/BP_FYW_Character.ClientEvent UpdateCountdown` _array_element_3 "1")
        (`/Game/CampusClash/Placeables/FindYourWay/BP_FYW_Character.ClientEvent PlaySound` _array_element_3 (`BlueprintMapLibrary.Map_Find` (`self.soundList`) "Countdown")))
      (`KismetSystemLibrary.Delay` 1.0)
      (if (`self.isGameOngoing`)
        (for _array_element_4 (`self.FYWCharacters`)
          (`/Game/CampusClash/Placeables/FindYourWay/BP_FYW_Character.ClientEvent StartRun` _array_element_4)
          (set `self.isRunOngoing` true)
          (`/Game/CampusClash/Placeables/FindYourWay/BP_FYW_Character.ClientEvent PlaySound` _array_element_4 (`BlueprintMapLibrary.Map_Find` (`self.soundList`) "RunStart")))
        (`KismetSystemLibrary.Delay` 1.0)
        (if (`self.isGameOngoing`)
          (for _array_element_5 (`self.FYWCharacters`)
            (`/Game/CampusClash/Placeables/FindYourWay/BP_FYW_Character.ClientEvent PlaySoundLooped` _array_element_5 (`BlueprintMapLibrary.Map_Find` (`self.soundList`) "Background"))))))))

(event `ServerEvent PlayerFinished`
  (params (player :type "/Game/CampusClash/Placeables/FindYourWay/BP_FYW_Character Object Reference"))
  (bind _victorydata (`self.victoryData`))
  (if (`self.isRunOngoing`)
    (set `self.isRunOngoing` false)
    (for _array_element (`self.FYWCharacters`)
      (`self.AddPlayerData` (== _array_element player) player))
    (for _array_element_2 (`self.FYWCharacters`)
      (if (== _array_element_2 player)
        (`/Game/CampusClash/Placeables/FindYourWay/BP_FYW_Character.ClientEvent RunFinished` _array_element_2 _victorydata "Winner")
        (`/Game/CampusClash/Placeables/FindYourWay/BP_FYW_Character.ClientEvent PlaySound` _array_element_2 "/Game/CampusClash/Sounds/SFX/MemoryGame/CardMatch/MiniGameWin_Cue1.MiniGameWin_Cue1")
        (`self.AddPoints` _array_element_2)
        (else
          (`/Game/CampusClash/Placeables/FindYourWay/BP_FYW_Character.ClientEvent RunFinished` _array_element_2 _victorydata "Loser")
          (`/Game/CampusClash/Placeables/FindYourWay/BP_FYW_Character.ClientEvent PlaySound` _array_element_2 "/Game/CampusClash/Sounds/SFX/MemoryGame/LosingMinigame_Cue.LosingMinigame_Cue"))))
    (`self.EndGame` player)))

(event `PlayerClickExit`
  (params (playerController :type "/Game/CampusClash/Core/Controllers/BP_PlayerController Object Reference"))
  (for _array_element (`self.FYWCharacters`)
    (`/Game/CampusClash/Placeables/FindYourWay/BP_FYW_Character.ClientEvent PlaySound` _array_element "/Game/CampusClash/Sounds/SFX/MemoryGame/MiniGame_GameCancelled_Cue.MiniGame_GameCancelled_Cue"))
  (bind _asbp_fyw_character (cast `/Game/CampusClash/Placeables/FindYourWay/BP_FYW_Character` (`Controller.K2_GetPawn` playerController)))
  (if (`self.isGameOngoing`)
    (`self.CancelGame`)
    (else
      (`self.PlayerReset` _asbp_fyw_character)
      (`self.RemovePlayerData` _asbp_fyw_character))))

(event `LoadNewLevel`
  (bind _levelnames (`self.levelNames`))
  (`GameplayStatics.UnloadStreamLevel` (`KismetStringLibrary.Conv_StringToName` (`self.loadedLevelName`)))
  (`KismetSystemLibrary.Delay` 0.5)
  (bind _output_get (set `self.loadedLevelName` (`|GetArrayItem` _levelnames (`KismetMathLibrary.RandomInteger` (`KismetArrayLibrary.Array_Length` _levelnames)))))
  (`GameplayStatics.LoadStreamLevel` (`KismetStringLibrary.Conv_StringToName` _output_get) true true)
  (`self.InitNewLevel`))

(event `PlayerDc`
  (params (pawn :type "/Game/CampusClash/Placeables/FindYourWay/BP_FYW_Character Object Reference"))
  (`self.DuplicatePawn` pawn)
  (if (`self.isGameOngoing`)
    (for (_array_element _array_index) (`self.FYWCharacters`)
      (if (== _array_element pawn)
        (`self.K2_DestroyActor` (`|GetArrayItem` (`self.players`) _array_index))
        (else
          (`/Game/CampusClash/Placeables/FindYourWay/BP_FYW_Character.ClientEvent PlaySound` _array_element "/Game/CampusClash/Sounds/SFX/MemoryGame/MiniGame_GameCancelled_Cue.MiniGame_GameCancelled_Cue"))))
    (`self.CancelGame`)
    (else
      (`self.RemovePlayerData` pawn)
      (`self.K2_DestroyActor` (`|GetArrayItem` (`self.players`))))))

(fn `AddPlayerData`
  (params (isWinner :type Boolean) (player :type "/Game/CampusClash/Placeables/FindYourWay/BP_FYW_Character Object Reference"))
  (locals (points :type Integer))
  (bind _playerstate (`Pawn.PlayerState` player))
  (bind _asbp_player_state (cast `/Game/CampusClash/Core/PlayerStates/BP_PlayerState` _playerstate))
  (if isWinner
    (bind _username (`/Game/CampusClash/Core/PlayerStates/BP_PlayerState.Username` _asbp_player_state))
    (`KismetArrayLibrary.Array_Add` (`self.victoryData`) (make `/Game/CampusClash/Core/Struct/STR_PlayerVictoryInfo` _playerstate "Winner" _username (`KismetTextLibrary.Conv_IntToText` (`self.pointsWinner`))))
    (else
      (`KismetArrayLibrary.Array_Add` (`self.victoryData`) (make `/Game/CampusClash/Core/Struct/STR_PlayerVictoryInfo` _playerstate "Loser" _username (`KismetTextLibrary.Conv_IntToText` 0))))))

(fn `AddPoints`
  (params (player :type "/Game/CampusClash/Placeables/FindYourWay/BP_FYW_Character Object Reference"))
  (bind _asbp_game_state (cast `/Game/CampusClash/Core/GameStates/BP_GameState` (`GameplayStatics.GetGameState`)))
  (bind _asbp_player_controller (cast `/Game/CampusClash/Core/Controllers/BP_PlayerController` (`Pawn.GetController` player)))
  (`/Game/CampusClash/Core/GameStates/BP_GameState.AddPoints` _asbp_game_state (`self.pointsWinner`) _asbp_player_controller))

(fn `CancelGame`
  (for _array_element (`self.FYWCharacters`)
    (if (`KismetSystemLibrary.IsValid` _array_element)
      (`/Game/CampusClash/Placeables/FindYourWay/BP_FYW_Character.ClientEvent CancelGame` _array_element)
      (`self.PlayerReset` _array_element)))
  (`self.Reset`))

(fn `DuplicatePawn`
  (params (pawn :type "/Game/CampusClash/Placeables/FindYourWay/BP_FYW_Character Object Reference"))
  (bind _returnvalue (`|SpawnActorFromClass` "/Game/CampusClash/Placeables/FindYourWay/BP_FYW_Character.BP_FYW_Character_C" (`self.GetTransform` pawn) "AlwaysSpawn" "MultiplyWithRoot" null null))
  (for (_array_element _array_index) (`self.FYWCharacters`)
    (if (== _array_element pawn)
      (`KismetArrayLibrary.Array_Set` (`self.FYWCharacters`) _array_index _returnvalue))))

(fn `EndGame`
  (params (winner :type "/Game/CampusClash/Placeables/FindYourWay/BP_FYW_Character Object Reference"))
  (for _array_element (`self.FYWCharacters`)
    (`/Game/CampusClash/Placeables/FindYourWay/BP_FYW_Character.ClientEvent EndGame` _array_element)
    (if (== _array_element winner)
      (`self.PlayerReset` _array_element true)))
  (`self.Reset`))

(fn `Initialize`
  (for _array_element (`self.interactables`)
    (add `/Game/CampusClash/Placeables/FindYourWay/BP_FYW_Interactable.OnPlayerJoin` _array_element (`|CreateDelegate` :!event `PlayerJoinEvent`))))

(fn `InitNewLevel`
  (bind _outactors (`GameplayStatics.GetAllActorsOfClass` "/Game/CampusClash/Placeables/FindYourWay/BP_FYW_Character.BP_FYW_Character_C"))
  (bind _output_get (set `self.FYWCharacters` _outactors))
  (set `self.maxPlayers` (`KismetArrayLibrary.Array_Length` _output_get))
  (for _array_element (`self.FYWCharacters`)
    (add `/Game/CampusClash/Placeables/FindYourWay/BP_FYW_Character.OnEnterFinish` _array_element (`|CreateDelegate` :!event `ServerEvent PlayerFinished`))
    (add `/Game/CampusClash/Placeables/FindYourWay/BP_FYW_Character.OnDc` _array_element (`|CreateDelegate` :!event `PlayerDc`)))
  (for _array_element_2 (`self.FYWCharacters`)
    (`KismetSystemLibrary.PrintString` (`KismetSystemLibrary.GetDisplayName` _array_element_2))))

(fn `PlayerJoin`
  (params (playerController :type "/Game/CampusClash/Core/Controllers/BP_PlayerController Object Reference"))
  (bind _joinedplayercount (`self.joinedPlayerCount`))
  (bind _output (`|GetArrayItem` (`self.FYWCharacters`) _joinedplayercount))
  (bind _output_2 (`|GetArrayItem` (`self.FYWCharacters`)))
  (bind _asbp_third_person_character (cast `/Game/StarterContent/ThirdPerson/Blueprints/BP_ThirdPersonCharacter` (`Controller.K2_GetPawn` playerController)))
  (`CharacterMovementComponent.DisableMovement` (`Character.CharacterMovement` _asbp_third_person_character))
  (add `/Game/CampusClash/Core/Controllers/BP_PlayerController.OnCPressed` playerController (`|CreateDelegate` :!event `PlayerClickExit`))
  (`KismetArrayLibrary.Array_Add` (`self.players`) _asbp_third_person_character)
  (`Controller.Possess` playerController _output)
  (if (== _joinedplayercount 0)
    (`/Game/CampusClash/Placeables/FindYourWay/BP_FYW_Character.Join` _output _asbp_third_person_character)
    (`/Engine/EditorBlueprintResources/StandardMacros.IncrementInt` (`self.joinedPlayerCount`))
    (else
      (`/Game/CampusClash/Placeables/FindYourWay/BP_FYW_Character.Join` _output _asbp_third_person_character)
      (bind _asbp_player_state (cast `/Game/CampusClash/Core/PlayerStates/BP_PlayerState` (`Pawn.PlayerState` _output_2)))
      (`/Game/CampusClash/Placeables/FindYourWay/BP_FYW_Character.ClientEvent AddOpponent` _output (`/Game/CampusClash/Core/PlayerStates/BP_PlayerState.Username` _asbp_player_state) (`|GetArrayItem` (`self.players`)))
      (bind _asbp_player_state_2 (cast `/Game/CampusClash/Core/PlayerStates/BP_PlayerState` (`Controller.PlayerState` (`Pawn.GetController` _output))))
      (`/Game/CampusClash/Placeables/FindYourWay/BP_FYW_Character.ClientEvent AddOpponent` _output_2 (`/Game/CampusClash/Core/PlayerStates/BP_PlayerState.Username` _asbp_player_state_2) (`|GetArrayItem` (`self.players`) 1))
      (`/Engine/EditorBlueprintResources/StandardMacros.IncrementInt` (`self.joinedPlayerCount`)
        (:`  `
          (`self.StartGame`))))))

(fn `PlayerReset`
  (params (player :type "/Game/CampusClash/Placeables/FindYourWay/BP_FYW_Character Object Reference") (isWinner :type Boolean))
  (locals (transformFactor :type "Float (double-precision)"))
  (bind _output (`|GetArrayItem` (`self.players`) (`KismetArrayLibrary.Array_Find` (`self.FYWCharacters`) player)))
  (clear `/Game/CampusClash/Placeables/FindYourWay/BP_FYW_Character.OnEnterFinish` player)
  (clear `/Game/CampusClash/Placeables/FindYourWay/BP_FYW_Character.OnDc` player)
  (bind _asbp_player_controller (cast `/Game/CampusClash/Core/Controllers/BP_PlayerController` (`Pawn.GetController` player)))
  (remove `/Game/CampusClash/Core/Controllers/BP_PlayerController.OnCPressed` _asbp_player_controller (`|CreateDelegate` :!event `PlayerClickExit`))
  (`Controller.Possess` _asbp_player_controller _output)
  (if isWinner
    (`/Game/StarterContent/ThirdPerson/Blueprints/BP_ThirdPersonCharacter.Multicast CastConfetti` _output)))

(fn `RemovePlayerData`
  (params (player :type "/Game/CampusClash/Placeables/FindYourWay/BP_FYW_Character Object Reference"))
  (bind _fywcharacters (`self.FYWCharacters`))
  (bind _returnvalue (`KismetArrayLibrary.Array_Find` _fywcharacters player))
  (`KismetArrayLibrary.Array_Remove` _fywcharacters _returnvalue)
  (`KismetArrayLibrary.Array_Remove` (`self.players`) _returnvalue)
  (`/Engine/EditorBlueprintResources/StandardMacros.DecrementInt` (`self.joinedPlayerCount`)))

(fn `Reset`
  (set `self.joinedPlayerCount` 0)
  (`KismetArrayLibrary.Array_Clear` (`self.players`))
  (`KismetArrayLibrary.Array_Clear` (`self.FYWCharacters`))
  (`self.LoadNewLevel`)
  (set `self.isGameOngoing` false)
  (set `self.isRunOngoing` false)
  (for _array_element (`self.interactables`)
    (set `/Game/CampusClash/Placeables/FindYourWay/BP_FYW_Interactable.isGameOngoing` false _array_element)
    (`KismetArrayLibrary.Array_Clear` (`self.victoryData`))))

(fn `StartGame`
  (set `self.isGameOngoing` true)
  (for _array_element (`self.interactables`)
    (set `/Game/CampusClash/Placeables/FindYourWay/BP_FYW_Interactable.isGameOngoing` true _array_element))
  (`self.HandleCountdown`))

(fn `UserConstructionScript`)