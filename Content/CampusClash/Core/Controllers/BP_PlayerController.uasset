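; Player controller for Campus Clash that sets up proximity voice chat with push-to-talk, plus debug and menu input.
; On BeginPlay it retries each tick until the PlayerState and pawn exist, then creates a VOIP talker attached to the character capsule with proximity attenuation.
; Debug keys toggle voice loopback, switch campus team and add points through the GameState.
; A key opens the options menu with game-and-UI input.
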(event `self.ReceiveBeginPlay`
  (bind _playerstate (`self.PlayerState`))
  ;[1 1 1] WIP Attach VOIP Talker to player collider
  (`/Engine/EditorBlueprintResources/StandardMacros.IsValid` _playerstate :!label _label
    (:`Is Valid`
      (bind _returnvalue (`VOIPTalker.CreateTalkerForPlayer` _playerstate))
      (set `self.VoipTalker` _returnvalue)
      (`VOIPStatics.SetMicThreshold` -2.0)
      (bind _asbp_third_person_character (cast `/Game/StarterContent/ThirdPerson/Blueprints/BP_ThirdPersonCharacter` (`self.K2_GetPawn`) :!label _label_2)
        (:`then`
          (set `VOIPTalker.Settings` (make `VoiceSettings` (`Character.CapsuleComponent` _asbp_third_person_character) "/Game/CampusClash/Sounds/Attenuations/ATT_ProximityVoice.ATT_ProximityVoice") (`self.VoipTalker`)))
        (:`CastFailed`
          (`KismetSystemLibrary.DelayUntilNextTick`)
          (goto _label_2))))
    (:`Is Not Valid`
      (`KismetSystemLibrary.DelayUntilNextTick`)
      (goto _label))))

(event `EnhancedInput|/Game/CampusClash/Core/Input/Actions/IA_PushToTalk`
  (params (ActionValue :type Boolean) (ElapsedSeconds :type "Float (double-precision)") (TriggeredSeconds :type "Float (double-precision)") (InputAction :type "InputAction Object Reference" :default "/Game/CampusClash/Core/Input/Actions/IA_PushToTalk.IA_PushToTalk"))
  ;[1 1 1] Push to Talk
  (:`Started`
    (`KismetSystemLibrary.PrintString` "Voice On")
    (`KismetSystemLibrary.ExecuteConsoleCommand` "ToggleSpeaking 1" null))
  (:`Completed`
    (`KismetSystemLibrary.PrintString` "Voice Off")
    (`KismetSystemLibrary.ExecuteConsoleCommand` "ToggleSpeaking 0" null)))

(event `Key|L`
  (params (Key :type "Key Structure"))
  ;[1 0.9647 0.02956] Debug loopback
  (:`Released`
    (bind _returnvalue (`KismetSystemLibrary.GetConsoleVariableBoolValue` "OSS.VoiceLoopback"))
    (if _returnvalue
      (`KismetSystemLibrary.ExecuteConsoleCommand` "OSS.VoiceLoopback 0" null)
      (`KismetSystemLibrary.PrintString` "Loopback 0" true true (struct :`G` 0.66 :`B` 1.0 :`A` 1.0) 10.0)
      (else
        (`KismetSystemLibrary.ExecuteConsoleCommand` "OSS.VoiceLoopback 1" null)
        (`KismetSystemLibrary.PrintString` "Loopback 1" true true (struct :`G` 0.66 :`B` 1.0 :`A` 1.0) 10.0)))))

(event `Key|NumPadOne`
  (params (Key :type "Key Structure"))
  ;[1 0.9668 0.03] DEBUG and testing functionality
  (:`Released`
    (bind _asbp_player_state (cast `/Game/CampusClash/Core/PlayerStates/BP_PlayerState` (`self.PlayerState`)))
    (`/Game/CampusClash/Core/PlayerStates/BP_PlayerState.SetCampusTeam` _asbp_player_state "NewEnumerator0")))

(event `Key|NumPadTwo`
  (params (Key :type "Key Structure"))
  ;[1 0.9668 0.03] DEBUG and testing functionality
  (:`Released`
    (bind _asbp_player_state (cast `/Game/CampusClash/Core/PlayerStates/BP_PlayerState` (`self.PlayerState`)))
    (`/Game/CampusClash/Core/PlayerStates/BP_PlayerState.SetCampusTeam` _asbp_player_state "NewEnumerator1")))

(event `Key|NumPadThree`
  (params (Key :type "Key Structure"))
  ;[1 0.9668 0.03] DEBUG and testing functionality
  (:`Released`
    (bind _asbp_player_state (cast `/Game/CampusClash/Core/PlayerStates/BP_PlayerState` (`self.PlayerState`)))
    (`/Game/CampusClash/Core/PlayerStates/BP_PlayerState.SetCampusTeam` _asbp_player_state "NewEnumerator2")))

(event `Key|NumPadNine`
  (params (Key :type "Key Structure"))
  ;[1 0.9668 0.03] DEBUG and testing functionality
  (:`Released`
    (`self.AddPoints`)))

(event `AddPoints`
  (bind _asbp_game_state (cast `/Game/CampusClash/Core/GameStates/BP_GameState` (`GameplayStatics.GetGameState`)))
  (`/Game/CampusClash/Core/GameStates/BP_GameState.AddPoints` _asbp_game_state 1 self))

(event `AddWidget`
  (params (newWidget :type "UserWidget Class Reference"))
  (bind _returnvalue (`|CreateWidget` newWidget self))
  (`UserWidget.AddToViewport` _returnvalue 0))

(event `Key|Two`
  (params (Key :type "Key Structure"))
  (:`Released`
    (`self.AddWidget` "/Game/CampusClash/Core/UI/EmotesUI/WBP_OptionMenu.WBP_OptionMenu_C")
    (set `self.bShowMouseCursor` true)
    (`WidgetBlueprintLibrary.SetInputMode_GameAndUIEx` self null "DoNotLock" false)))

(fn `UserConstructionScript`)