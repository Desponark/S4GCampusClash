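; Player-side Blueprint for the Memory card minigame, handling card picking, per-player UI and sound in a networked match.
; A left click traces under the cursor and sends any hit BP_Card to the server, which notifies the card.
; Client events manage the HUD, score and turn text, result screen, cursor visibility and sounds, including one replaceable loop.
; Exit requests fire the OnClickExit dispatcher, and Reset clears pair count, clicked card and HUD.
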(event `EnhancedInput|/Game/CampusClash/Core/Input/Actions/IA_LeftClick`
  (params (ActionValue :type Boolean) (ElapsedSeconds :type "Float (double-precision)") (TriggeredSeconds :type "Float (double-precision)") (InputAction :type "InputAction Object Reference" :default "/Game/CampusClash/Core/Input/Actions/IA_LeftClick.IA_LeftClick"))
  (:`Completed`
    (bind _hitactor (`self.GetActorUnderMouse`))
    (bind _asbp_card (cast `/Game/CampusClash/Placeables/MemoryGame/BP_Card` _hitactor))
    (`self.ServerEvent OnCardSelected` _asbp_card)))

(event `ServerEvent OnCardSelected`
  (params (card :type "/Game/CampusClash/Placeables/MemoryGame/BP_Card Object Reference"))
  (`/Game/CampusClash/Placeables/MemoryGame/BP_Card.CardSelected` card self))

(event `ClientEvent InitMainWidget`
  (params (memoryGame :type "/Game/CampusClash/Placeables/MemoryGame/BP_MemoryGame Object Reference"))
  (bind _localjoinwidget (`/Game/CampusClash/Placeables/MemoryGame/BP_MemoryGame.localJoinWidget` memoryGame))
  (`KismetSystemLibrary.PrintString` "init main widget")
  (if (`KismetSystemLibrary.IsValid` _localjoinwidget)
    (`Widget.RemoveFromParent` _localjoinwidget))
  (bind _asbp_player_controller (cast `/Game/CampusClash/Core/Controllers/BP_PlayerController` (`self.GetController` self)))
  (bind _returnvalue (`|CreateWidget` "/Game/CampusClash/Core/UI/WBP_PlayerHUDMemory.WBP_PlayerHUDMemory_C" _asbp_player_controller))
  (bind _output_get (set `self.mainWidget` _returnvalue))
  (`UserWidget.AddToViewport` _output_get 0)
  (set `PlayerController.bShowMouseCursor` true _asbp_player_controller))

(event `ClientEvent UpdateScoreUI`
  (params (yourScore :type Integer) (opponentScore :type Integer))
  (`TextBlock.SetText` (`/Game/CampusClash/Core/UI/WBP_PlayerHUDMemory.Player1PairsCount` (`self.mainWidget`)) (`KismetTextLibrary.Conv_IntToText` yourScore))
  (`TextBlock.SetText` (`/Game/CampusClash/Core/UI/WBP_PlayerHUDMemory.Player2PairsCount` (`self.mainWidget`)) (`KismetTextLibrary.Conv_IntToText` opponentScore)))

(event `ClientEvent UpdateTurnInfo`
  (params (turnInfo :type String))
  (`TextBlock.SetText` (`/Game/CampusClash/Core/UI/WBP_PlayerHUDMemory.TurnInfo` (`self.mainWidget`)) (`KismetTextLibrary.Conv_StringToText` turnInfo)))

(event `ClientEvent Exit`
  (bind _activesoundloop (`self.activeSoundLoop`))
  (`Widget.RemoveFromParent` (`self.mainWidget`))
  (bind _asbp_player_controller (cast `/Game/CampusClash/Core/Controllers/BP_PlayerController` (`self.GetController` self)))
  (set `PlayerController.bShowMouseCursor` false _asbp_player_controller)
  (`AudioComponent.Stop` _activesoundloop)
  (`ActorComponent.K2_DestroyComponent` _activesoundloop))

(event `ServerEvent ClickExit`
  (`self.OnClickExit` self))

(event `ClientEvent InitResultWidget`
  (params (result :type String))
  (bind _asbp_player_controller (cast `/Game/CampusClash/Core/Controllers/BP_PlayerController` (`GameplayStatics.GetPlayerController` 0)))
  (bind _returnvalue (`|CreateWidget` "/Game/CampusClash/Placeables/MemoryGame/WBP_Memory_EndScreen.WBP_Memory_EndScreen_C" _asbp_player_controller))
  (`TextBlock.SetText` (`/Game/CampusClash/Placeables/MemoryGame/WBP_Memory_EndScreen.Result` _returnvalue) (`KismetTextLibrary.Conv_StringToText` result))
  (`UserWidget.AddToViewport` _returnvalue 0))

(event `ClientEvent PlaySound`
  (params (sound :type "SoundCue Object Reference"))
  (`GameplayStatics.PlaySound2D` sound 1.0 1.0 0.0 null null))

(event `ClientEvent PlaySoundLooped`
  (params (sound :type "SoundCue Object Reference"))
  (bind _activesoundloop (`self.activeSoundLoop`))
  (if (`KismetSystemLibrary.IsValid` (`self.activeSoundLoop`))
    (`AudioComponent.Stop` _activesoundloop)
    (`ActorComponent.K2_DestroyComponent` _activesoundloop)
    (bind _returnvalue (`GameplayStatics.SpawnSound2D` sound 1.0 1.0 0.0 null false false))
    (set `self.activeSoundLoop` _returnvalue)
    (else
      (bind _returnvalue_2 (`GameplayStatics.SpawnSound2D` sound 1.0 1.0 0.0 null false false))
      (set `self.activeSoundLoop` _returnvalue_2))))

(fn `GetActorUnderMouse`
  (returns (hitActor :type "Actor Object Reference"))
  (bind _returnvalue (`GameplayStatics.GetPlayerController` 0))
  (if (`KismetSystemLibrary.IsValid` _returnvalue)
    (return (`.HitActor` (`GameplayStatics.BreakHitResult` (`PlayerController.GetHitResultUnderCursorByChannel` _returnvalue "TraceTypeQuery2" true))))))

(fn `Reset`
  (bind _mainwidget (`self.mainWidget`))
  (set `self.gatheredPairCount` 0)
  (set `self.clickedCard` null)
  (if (`KismetSystemLibrary.IsValid` _mainwidget)
    (`Widget.RemoveFromParent` _mainwidget)))

(fn `UserConstructionScript`)