(event `self.Box.OnComponentBeginOverlap`
  (params (OverlappedComponent :type "PrimitiveComponent Object Reference") (OtherActor :type "Actor Object Reference") (OtherComp :type "PrimitiveComponent Object Reference") (OtherBodyIndex :type Integer) (bFromSweep :type Boolean) (SweepResult :type "HitResult Structure (by ref)")))

(event `self.Box.OnComponentEndOverlap`
  (params (OverlappedComponent :type "PrimitiveComponent Object Reference") (OtherActor :type "Actor Object Reference") (OtherComp :type "PrimitiveComponent Object Reference") (OtherBodyIndex :type Integer)))

(event `/Game/CampusClash/Core/Interaction/BPI_Interaction.OnInteraction`
  (params (InteractingPlayer :type "Actor Object Reference"))
  (bind _asbp_third_person_character (cast `/Game/StarterContent/ThirdPerson/Blueprints/BP_ThirdPersonCharacter` InteractingPlayer))
  (if (`self.isGameOngoing`)
    (bind _asbp_player_controller (cast `/Game/CampusClash/Core/Controllers/BP_PlayerController` (`Pawn.GetController` _asbp_third_person_character)))
    (bind _returnvalue (`|CreateWidget` "/Game/CampusClash/Core/UI/MiniGames/WBP_GameStateInfo.WBP_GameStateInfo_C" _asbp_player_controller))
    (`/Game/CampusClash/Core/UI/MiniGames/WBP_GameStateInfo.DelayedDestroy` _returnvalue)
    (`UserWidget.AddToViewport` _returnvalue 0)
    (else
      (`self.OnPlayerJoin` _asbp_third_person_character))))

(fn `InteractionPrompt`
  (returns (IsEnabled :type Boolean) (Text :type Text))
  (if (`self.isGameOngoing`)
    (return true "Game has already started ")
    (else
      (return true "to play"))))

(fn `UserConstructionScript`)