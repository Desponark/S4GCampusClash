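; Player-side actor for the TicTacToe minigame, relaying between the game and the player's UI.
; Client events manage the HUD, mouse cursor, turn text, board interactability, category display and 2D sounds, including one replaceable loop.
; Server events forward field and exit clicks through CallOnClickField and CallOnClickExit.
; The result screen reuses the Memory end-screen widget, and the left-click cursor trace result is unused.
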(event `Initialize`
  (params (game :type "/Game/CampusClash/Placeables/TicTacToeGame/BP_TicTacToe_Game Object Reference"))
  (set `self.gameWidget` (`/Game/CampusClash/Placeables/TicTacToeGame/BP_TicTacToe_Game.gameWidget` game))
  (`/Game/CampusClash/Placeables/TicTacToeGame/BP_TicTacToe_Game.InitGameWidget` game self))

(event `EnhancedInput|/Game/CampusClash/Core/Input/Actions/IA_LeftClick`
  (params (ActionValue :type Boolean) (ElapsedSeconds :type "Float (double-precision)") (TriggeredSeconds :type "Float (double-precision)") (InputAction :type "InputAction Object Reference" :default "/Game/CampusClash/Core/Input/Actions/IA_LeftClick.IA_LeftClick"))
  (:`Completed`
    (`self.GetActorUnderMouse`)))

(event `ClientEvent UpdateTurnInfo`
  (params (turnInfo :type String))
  (`TextBlock.SetText` (`/Game/CampusClash/Core/UI/WBP_Player_HUDTicTacToe.TurnInfo` (`self.playerWidget`)) (`KismetTextLibrary.Conv_StringToText` turnInfo)))

(event `ClientEvent DeactivateInput`
  (params (game :type "/Game/CampusClash/Placeables/TicTacToeGame/BP_TicTacToe_Game Object Reference"))
  (`/Game/CampusClash/Placeables/TicTacToeGame/BP_TicTacToe_Game.SetInteractability` game false))

(event `ClientEvent ActivateInput`
  (params (game :type "/Game/CampusClash/Placeables/TicTacToeGame/BP_TicTacToe_Game Object Reference"))
  (`/Game/CampusClash/Placeables/TicTacToeGame/BP_TicTacToe_Game.SetInteractability` game true))

(event `ClientEvent Exit`
  (bind _activesoundloop (`self.activeSoundLoop`))
  (`Widget.RemoveFromParent` (`self.playerWidget`))
  (bind _asbp_player_controller (cast `/Game/CampusClash/Core/Controllers/BP_PlayerController` (`self.GetController` self)))
  (set `PlayerController.bShowMouseCursor` false _asbp_player_controller)
  (`AudioComponent.Stop` _activesoundloop)
  (`ActorComponent.K2_DestroyComponent` _activesoundloop))

(event `ClientEvent InitPlayerWidget`
  (bind _asbp_player_controller (cast `/Game/CampusClash/Core/Controllers/BP_PlayerController` (`self.GetController` self)))
  (bind _returnvalue (`|CreateWidget` "/Game/CampusClash/Core/UI/WBP_Player_HUDTicTacToe.WBP_Player_HUDTicTacToe_C" _asbp_player_controller))
  (bind _output_get (set `self.playerWidget` _returnvalue))
  (`UserWidget.AddToViewport` _output_get 0)
  (set `PlayerController.bShowMouseCursor` true _asbp_player_controller))

(event `ClientEvent InitResultWidget`
  (params (result :type String))
  (bind _asbp_player_controller (cast `/Game/CampusClash/Core/Controllers/BP_PlayerController` (`GameplayStatics.GetPlayerController` 0)))
  (bind _returnvalue (`|CreateWidget` "/Game/CampusClash/Core/UI/HUDs/WBP_Memory_EndScreen.WBP_Memory_EndScreen_C" _asbp_player_controller))
  (`TextBlock.SetText` (`/Game/CampusClash/Core/UI/HUDs/WBP_Memory_EndScreen.Result` _returnvalue) (`KismetTextLibrary.Conv_StringToText` result))
  (`UserWidget.AddToViewport` _returnvalue 0))

(event `ClientEvent PlaySound`
  (params (sound :type "SoundCue Object Reference"))
  (`GameplayStatics.PlaySound2D` sound 1.0 1.0 0.0 null null))

(event `ClientEvent PlaySoundLooped`
  (params (sound :type "SoundCue Object Reference"))
  (bind _activesoundloop (`self.activeSoundLoop`))
  (if (`KismetSystemLibrary.IsValid` (`self.activeSoundLoop`))
    (`AudioComponent.Stop` _activesoundloop)
    (`ActorComponent.K2_DestroyComponent` _activesoundloop)
    (bind _returnvalue (`GameplayStatics.SpawnSound2D` sound 1.0 1.0 0.0 null false false))
    (set `self.activeSoundLoop` _returnvalue)
    (else
      (bind _returnvalue_2 (`GameplayStatics.SpawnSound2D` sound 1.0 1.0 0.0 null false false))
      (set `self.activeSoundLoop` _returnvalue_2))))

(event `ClientEvent UpdateFields`
  (params (game :type "/Game/CampusClash/Placeables/TicTacToeGame/BP_TicTacToe_Game Object Reference"))
  (`/Game/CampusClash/Placeables/TicTacToeGame/BP_TicTacToe_Game.ShowCategories` game))

(event `ServerEvent ClickExit`
  (`self.OnClickExit` self))

(event `ServerEvent ClickField`
  (params (index :type Integer))
  (`KismetSystemLibrary.PrintString` "call on player")
  (`self.OnClickField` index))

(event `ClickField`
  (`KismetSystemLibrary.PrintString` "client event on player")
  (`self.ServerEvent ClickField` 0))

(fn `GetActorUnderMouse`
  (returns (hitActor :type "Actor Object Reference"))
  (bind _returnvalue (`GameplayStatics.GetPlayerController` 0))
  (if (`KismetSystemLibrary.IsValid` _returnvalue)
    (return (`.HitActor` (`GameplayStatics.BreakHitResult` (`PlayerController.GetHitResultUnderCursorByChannel` _returnvalue "TraceTypeQuery2" true))))))

(fn `Reset`)

(fn `UserConstructionScript`)