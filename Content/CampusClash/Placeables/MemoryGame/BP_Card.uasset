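; BP_Card is a placeable card for the Campus Clash memory game that is assigned a material, starts rolled 180 degrees and reports selection through an event dispatcher.
; Open and Hide set a RepNotify state, and either value triggers Turn, which chains three timelines to lift, roll and lower the card.
; The material is also RepNotify and is applied to the cube on change, while hover events scale the card up and back.
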(event `CardSelected`
  (params (player :type "/Game/CampusClash/Placeables/MemoryGame/BP_MemoryPlayer Object Reference"))
  (`KismetSystemLibrary.PrintString` "call card selected in card" true true (struct :`G` 0.66 :`B` 1.0 :`A` 1.0) 5.0)
  (`self.OnCardSelected` self player))

(event `Initialize`
  (params (material :type "MaterialInstance Object Reference"))
  (bind (_returnvalue_roll _returnvalue_pitch _returnvalue_yaw) (`KismetMathLibrary.BreakRotator` (`self.K2_GetActorRotation`)))
  (set `self.material` material)
  (`self.K2_SetActorRotation` (`KismetMathLibrary.MakeRotator` 180.0 _returnvalue_pitch _returnvalue_yaw)))

(event `Open`
  (set `self.state` "NewEnumerator1"))

(event `Hide`
  (set `self.state` "NewEnumerator2"))

(event `Turn`
  (bind (_startrotation_roll _startrotation_pitch _startrotation_yaw) (`KismetMathLibrary.BreakRotator` (`self.startRotation`)))
  (bind (_startlocation_x _startlocation_y _startlocation_z) (`KismetMathLibrary.BreakVector` (`self.startLocation`)))
  (bind (_startlocation_x_2 _startlocation_y_2 _startlocation_z_2) (`KismetMathLibrary.BreakVector` (`self.startLocation`)))
  (set `self.startLocation` (`self.K2_GetActorLocation`))
  (bind (_direction _newtrack_1) (`Timeline|Up` :!via `PlayFromStart`)
    (:`Update`
      (`self.K2_SetActorLocation` (`KismetMathLibrary.MakeVector` _startlocation_x_2 _startlocation_y_2 (+ _startlocation_z_2 _newtrack_1))))
    (:`Finished`
      (set `self.startRotation` (`self.K2_GetActorRotation`))
      (bind (_direction_2 _newtrack_0) (`Timeline|TurnAround` :!via `PlayFromStart`)
        (:`Update`
          (`self.K2_SetActorRotation` (`KismetMathLibrary.MakeRotator` (+ _newtrack_0 _startrotation_roll) _startrotation_pitch _startrotation_yaw)))
        (:`Finished`
          (set `self.startLocation` (`self.K2_GetActorLocation`))
          (bind (_direction_3 _newtrack_1_2) (`Timeline|Timeline` :!via `PlayFromStart`)
            (:`Update`
              (`self.K2_SetActorLocation` (`KismetMathLibrary.MakeVector` _startlocation_x _startlocation_y (- _startlocation_z _newtrack_1_2))))))))))

(event `StartHover`
  (set `self.hoveredOver` true)
  (`self.SetActorScale3D` (* (`self.GetActorScale3D`) (`self.hoveredScale`))))

(event `StopHover`
  (set `self.hoveredOver` false)
  (`self.SetActorScale3D` (/ (`self.GetActorScale3D`) (`self.hoveredScale`))))

(fn `OnRep_material`
  (`PrimitiveComponent.SetMaterial` (`self.Cube`) 0 (`self.material`)))

(fn `OnRep_state`
  (switch `/Game/CampusClash/Core/Struct/EMemoryCardState` (`self.state`)
    (:`NewEnumerator1`
      _)
    (:`NewEnumerator2`
      _))
  (`self.Turn`))

(fn `UserConstructionScript`)