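; Player state for CampusClash that holds each player's campus team and username and carries both through seamless travel via CopyProperties.
; Team and name setters update the pawn's BP_ThirdPersonCharacter antenna visibility and name tag, with team changes also printing a debug message.
; A collectible function marks an array entry as unlocked and shows an alert widget, while InteractionPrompt returns a disabled, empty prompt.
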(event `SetCampusTeam`
  (params (NewTeam :type "/Game/CampusClash/Core/Enums/ECampusTeam Enum" :default "NewEnumerator0"))
  (bind _output_get (set `self.CampusTeam` NewTeam))
  (`KismetSystemLibrary.PrintText` (`|FormatText` "Set Team to {Team}" (`|GetEnumeratorNameAsString` _output_get)) true true (struct :`R` 0.217397 :`G` 0.69 :`A` 1.0) 4.0)
  (bind _asbp_third_person_character (cast `/Game/StarterContent/ThirdPerson/Blueprints/BP_ThirdPersonCharacter` (`self.GetPawn`)))
  (`/Game/StarterContent/ThirdPerson/Blueprints/BP_ThirdPersonCharacter.SetAntennaVisibility` _asbp_third_person_character _output_get))

(event `self.ReceiveCopyProperties`
  (params (NewPlayerState :type "PlayerState Object Reference"))
  ;[1 1 1] Copy props for seamless travel
  (bind _asbp_player_state (cast `/Game/CampusClash/Core/PlayerStates/BP_PlayerState` NewPlayerState))
  (set `/Game/CampusClash/Core/PlayerStates/BP_PlayerState.CampusTeam` (`self.CampusTeam`) _asbp_player_state)
  (set `/Game/CampusClash/Core/PlayerStates/BP_PlayerState.Username` (`self.Username`) _asbp_player_state))

(event `SetUserName`
  (params (Username :type Text))
  (set `self.Username` Username)
  (bind _asbp_third_person_character (cast `/Game/StarterContent/ThirdPerson/Blueprints/BP_ThirdPersonCharacter` (`self.GetPawn`)))
  (`/Game/StarterContent/ThirdPerson/Blueprints/BP_ThirdPersonCharacter.UpdateNameTag` _asbp_third_person_character))

(fn `InteractionPrompt`
  (returns (IsEnabled :type Boolean) (Text :type Text))
  (return false ""))

(fn `Set Collectible As Got`
  (params (Index :type Integer))
  (locals (NewLocalVar_0 :type Boolean :default false))
  (bind _collectible_collactables (break `/Game/CampusClash/Core/Struct/STR_Collectables` (`self.Collectible`)))
  (bind _collectible_collactables_2 (break `/Game/CampusClash/Core/Struct/STR_Collectables` (`self.Collectible`)))
  (bind (_name _imgunlocked _imglocked) (break `/Game/CampusClash/Core/Struct/STR_Collectable` (`|GetArrayItem` _collectible_collactables_2 Index)))
  (`KismetArrayLibrary.Array_Set` _collectible_collactables Index (make `/Game/CampusClash/Core/Struct/STR_Collectable` _name _imgunlocked _imglocked true))
  (bind _returnvalue (`|CreateWidget` "/Game/CampusClash/Core/UI/CollectibleUI/WBP_CollectibleAlert.WBP_CollectibleAlert_C"))
  (`UserWidget.AddToViewport` _returnvalue 0))

(fn `UserConstructionScript`)