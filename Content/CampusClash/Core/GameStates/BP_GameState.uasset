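; Game state for Campus Clash that keeps the point totals for the Hamburg and Berlin campus teams.
; AddPoints reads the campus team from the given controller's player state and adds the points to that team's total.
; Both totals use RepNotify functions that fire UpdatePoints with the changed team, so listeners can react to score changes.
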(event `AddPoints`
  (params (Points :type Integer) (PlayerController :type "/Game/CampusClash/Core/Controllers/BP_PlayerController Object Reference"))
  (bind _asbp_player_state (cast `/Game/CampusClash/Core/PlayerStates/BP_PlayerState` (`Controller.PlayerState` PlayerController)))
  (switch `/Game/CampusClash/Core/Enums/ECampusTeam` (`/Game/CampusClash/Core/PlayerStates/BP_PlayerState.CampusTeam` _asbp_player_state)
    (:`NewEnumerator1`
      (set `self.HamburgPoints` (+ Points (`self.HamburgPoints`))))
    (:`NewEnumerator2`
      (set `self.BerlinPoints` (+ Points (`self.BerlinPoints`))))))

(fn `OnRep_BerlinPoints`
  (`self.UpdatePoints` "NewEnumerator2"))

(fn `OnRep_HamburgPoints`
  (`self.UpdatePoints` "NewEnumerator1"))

(fn `UserConstructionScript`)