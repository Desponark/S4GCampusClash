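; Double door for Campus Clash that opens when a third-person character enters its trigger box and closes when the last one leaves.
; An overlap counter tracks characters in the box, so the door only starts opening for the first and closing after the last.
; One Timeline plays forward or in reverse, moving the two door meshes' relative locations on separate tracks, with the same sound played each way.
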(event `self.Box.OnComponentBeginOverlap`
  (params (OverlappedComponent :type "PrimitiveComponent Object Reference") (OtherActor :type "Actor Object Reference") (OtherComp :type "PrimitiveComponent Object Reference") (OtherBodyIndex :type Integer) (bFromSweep :type Boolean) (SweepResult :type "HitResult Structure (by ref)"))
  (cast `/Game/StarterContent/ThirdPerson/Blueprints/BP_ThirdPersonCharacter` OtherActor)
  (bind _result (`/Engine/EditorBlueprintResources/StandardMacros.IncrementInt` (`self.Counter`))
    (:`  `
      (if (<= _result 1)
        (`GameplayStatics.PlaySoundAtLocation` "/Game/CampusClash/Sounds/SFX/DoorOpen_Close.DoorOpen_Close" (`self.K2_GetActorLocation`) (struct) 1.0 1.0 0.0 "/Game/CampusClash/Sounds/Attenuations/ATT_Door.ATT_Door" null null null)
        (bind (_direction _newtrack_0 _newtrack_1) (`Timeline|Timeline` :!label _label)
          (:`Update`
            (`SceneComponent.K2_SetRelativeLocation` (`self.CampusSingleDoorMesh`) _newtrack_0 false false)
            (`SceneComponent.K2_SetRelativeLocation` (`self.CampusSingleDoorMesh1`) _newtrack_1 false false)))))))

(event `self.Box.OnComponentEndOverlap`
  (params (OverlappedComponent :type "PrimitiveComponent Object Reference") (OtherActor :type "Actor Object Reference") (OtherComp :type "PrimitiveComponent Object Reference") (OtherBodyIndex :type Integer))
  (cast `/Game/StarterContent/ThirdPerson/Blueprints/BP_ThirdPersonCharacter` OtherActor)
  (bind _result (`/Engine/EditorBlueprintResources/StandardMacros.DecrementInt` (`self.Counter`))
    (:`  `
      (if (<= _result 0)
        (`GameplayStatics.PlaySoundAtLocation` "/Game/CampusClash/Sounds/SFX/DoorOpen_Close.DoorOpen_Close" (`self.K2_GetActorLocation`) (struct) 1.0 1.0 0.0 "/Game/CampusClash/Sounds/Attenuations/ATT_Door.ATT_Door" null null null)
        (goto _label :!via `Reverse`)))))

(fn `UserConstructionScript`)