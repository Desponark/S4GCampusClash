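; BP_DrinksMachine is an interactable vending machine placeable that dispenses a random drink can for a player character.
; Interaction calls ActivateDrinksMachineALL, which checks for BP_ThirdPersonCharacter and uses a DoOnce to block repeat use during dispensing.
; It plays coin and drop sounds with a machine animation, separated by delays.
; It then spawns a Mate or RedCrab can at SpawnPos, impulses it forward and resets the gate.
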(event `/Game/CampusClash/Core/Interaction/BPI_Interaction.OnInteraction`
  (params (InteractingPlayer :type "Actor Object Reference"))
  (`self.ActivateDrinksMachineALL` InteractingPlayer))

(event `ActivateDrinksMachineALL`
  (params (Object :type "Object Object Reference"))
  (bind (_returnvalue_location _returnvalue_rotation) (`KismetMathLibrary.BreakTransform` (`SceneComponent.K2_GetComponentToWorld` (`self.SpawnPos`))))
  (bind _returnvalue (* (`SceneComponent.GetForwardVector` (`self.SpawnPos`)) 100.0))
  (cast `/Game/StarterContent/ThirdPerson/Blueprints/BP_ThirdPersonCharacter` Object)
  (`/Engine/EditorBlueprintResources/StandardMacros.DoOnce` false :!label _label
    (:`Completed`
      (`GameplayStatics.PlaySoundAtLocation` "/Game/CampusClash/Sounds/SFX/DrinkMachine/MoneyDropIn_Cue.MoneyDropIn_Cue" (`self.K2_GetActorLocation`) (struct) 1.0 1.0 0.0 "/Game/CampusClash/Sounds/Attenuations/ATT_Door.ATT_Door" null null null)
      (`KismetSystemLibrary.Delay` 1.0)
      (`SkeletalMeshComponent.PlayAnimation` (`self.SK_DrinkMachine`) "/Game/CampusClash/Art/Assets/DrinkMachine/New/A_DrinkMachine.A_DrinkMachine" false)
      (`GameplayStatics.PlaySoundAtLocation` "/Game/CampusClash/Sounds/SFX/DrinkMachine/DrinkMachineDropOut.DrinkMachineDropOut" (`self.K2_GetActorLocation`) (struct) 1.0 1.0 0.0 "/Game/CampusClash/Sounds/Attenuations/ATT_Door.ATT_Door" null null null)
      (`KismetSystemLibrary.Delay` 3.5)
      (if (`KismetMathLibrary.RandomBool`)
        (bind _returnvalue_2 (`|SpawnActorFromClass` "/Game/CampusClash/Placeables/DrinksMachine/BP_DrinkMateDrop.BP_DrinkMateDrop_C" (`KismetMathLibrary.MakeTransform` _returnvalue_location _returnvalue_rotation) "Undefined" "MultiplyWithRoot" null null))
        (`PrimitiveComponent.AddImpulse` (`/Game/CampusClash/Placeables/DrinksMachine/BP_DrinkMateDrop.NoyanMateCan2` _returnvalue_2) _returnvalue "None" false)
        (goto _label :!via `Reset`)
        (else
          (bind _returnvalue_3 (`|SpawnActorFromClass` "/Game/CampusClash/Placeables/DrinksMachine/BP_DrinkRedCrabDrop.BP_DrinkRedCrabDrop_C" (`KismetMathLibrary.MakeTransform` _returnvalue_location _returnvalue_rotation) "Undefined" "MultiplyWithRoot" null null))
          (`PrimitiveComponent.AddImpulse` (`/Game/CampusClash/Placeables/DrinksMachine/BP_DrinkRedCrabDrop.RedCrabCan2` _returnvalue_3) _returnvalue "None" false)
          (goto _label :!via `Reset`))))))

(fn `InteractionPrompt`
  (returns (IsEnabled :type Boolean) (Text :type Text))
  (return true "to interact"))

(fn `UserConstructionScript`)