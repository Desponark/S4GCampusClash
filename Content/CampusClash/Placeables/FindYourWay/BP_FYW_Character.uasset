(event `Multicast Join`
  (bind _aswbp_name_tag (cast `/Game/CampusClash/Core/UI/NameTag/WBP_NameTag` (`WidgetComponent.GetWidget` (`self.NameTagWidget`))))
  (set `TextBlock.Text` "" (`/Game/CampusClash/Core/UI/NameTag/WBP_NameTag.Name` _aswbp_name_tag)))

(event `Join`
  (params (mainChar :type "/Game/StarterContent/ThirdPerson/Blueprints/BP_ThirdPersonCharacter Object Reference"))
  (`CharacterMovementComponent.DisableMovement` (`self.CharacterMovement`))
  (`self.Multicast Join`)
  (`self.ClientEvent Join` mainChar))

(event `ClientEvent Join`
  (params (mainChar :type "/Game/StarterContent/ThirdPerson/Blueprints/BP_ThirdPersonCharacter Object Reference"))
  (bind _returnvalue (`GameplayStatics.GetPlayerController` 0))
  (bind _returnvalue_2 (`|CreateWidget` "/Game/CampusClash/Core/UI/MiniGames/Memory/WBP_PlayerHUD_FYW.WBP_PlayerHUD_FYW_C" _returnvalue))
  (bind _asbp_player_state (cast `/Game/CampusClash/Core/PlayerStates/BP_PlayerState` (`Controller.PlayerState` _returnvalue)))
  (bind _rendermaterialbody (`self.CreateRenderMaterialHead` mainChar))
  (`/Game/CampusClash/Core/UI/MiniGames/Memory/WBP_PlayerHUD_FYW.AddOwningPlayer` _returnvalue_2 (`/Game/CampusClash/Core/PlayerStates/BP_PlayerState.Username` _asbp_player_state) _rendermaterialbody)
  (bind _output_get (set `self.gameWidget` _returnvalue_2))
  (`UserWidget.AddToViewport` _output_get 0)
  (`SceneComponent.SetVisibility` (`self.Mesh`) false true))

(event `ClientEvent AddOpponent`
  (params (opponentName :type Text) (mainChar :type "/Game/StarterContent/ThirdPerson/Blueprints/BP_ThirdPersonCharacter Object Reference"))
  (bind _rendermaterialbody (`self.CreateRenderMaterialHead` mainChar))
  (`/Game/CampusClash/Core/UI/MiniGames/Memory/WBP_PlayerHUD_FYW.AddOpponent` (`self.gameWidget`) opponentName _rendermaterialbody))

(event `ClientEvent StartCountdown`
  (`self.InitCountdownWidget`))

(event `ClientEvent UpdateCountdown`
  (params (countdown :type String))
  (`TextBlock.SetText` (`/Game/CampusClash/Core/UI/MiniGames/FindYourWay/WBP_FYW_Countdown.countdown` (`self.countdownWidget`)) (`KismetTextLibrary.Conv_StringToText` countdown)))

(event `ClientEvent StartRun`
  (set `self.startTime` (`GameplayStatics.GetTimeSeconds`))
  (`self.DestroyWidget` (`self.countdownWidget`))
  (`self.ServerEvent StartRun`))

(event `ServerEvent StartRun`
  (`CharacterMovementComponent.SetMovementMode` (`self.CharacterMovement`) "MOVE_Walking" 0))

(event `ClientEvent EndGame`
  (bind _activesoundloop (`self.activeSoundLoop`))
  (`self.DestroyWidget` (`self.endWidget`))
  (`self.DestroyWidget` (`self.gameWidget`))
  (`AudioComponent.Stop` _activesoundloop)
  (`ActorComponent.K2_DestroyComponent` _activesoundloop)
  (`SceneComponent.SetVisibility` (`self.Mesh`) true true))

(event `ClientEvent CancelGame`
  (bind _activesoundloop (`self.activeSoundLoop`))
  (`self.DestroyWidget` (`self.gameWidget`))
  (`self.DestroyWidget` (`self.countdownWidget`))
  (`self.DestroyWidget` (`self.endWidget`))
  (if (`KismetSystemLibrary.IsValid` _activesoundloop)
    (`AudioComponent.Stop` _activesoundloop)
    (`ActorComponent.K2_DestroyComponent` _activesoundloop)
    (`SceneComponent.SetVisibility` (`self.Mesh`) true true)))

(event `self.InteractionCollider.OnComponentBeginOverlap`
  (params (OverlappedComponent :type "PrimitiveComponent Object Reference") (OtherActor :type "Actor Object Reference") (OtherComp :type "PrimitiveComponent Object Reference") (OtherBodyIndex :type Integer) (bFromSweep :type Boolean) (SweepResult :type "HitResult Structure (by ref)"))
  (bind _asbp_fyw_finish (cast `/Game/CampusClash/Placeables/FindYourWay/BP_FYW_Finish` OtherActor))
  (if (== _asbp_fyw_finish (`self.finish`))
    (`self.ServerEvent CallOnEnterFinish`)))

(event `ServerEvent CallOnEnterFinish`
  (`self.OnEnterFinish` self))

(event `ClientEvent DestroyJoinWidget`
  (params (interactable :type "/Game/CampusClash/Placeables/FindYourWay/BP_FYW_Interactable Object Reference"))
  (if (`KismetSystemLibrary.IsValid` interactable)
    (`Widget.RemoveFromParent` (`/Game/CampusClash/Placeables/FindYourWay/BP_FYW_Interactable.localJoinWidget` interactable))))

(event `ClientEvent PlaySound`
  (params (sound :type "SoundCue Object Reference"))
  (`GameplayStatics.PlaySound2D` sound 1.0 1.0 0.0 null null))

(event `ClientEvent PlaySoundLooped`
  (params (sound :type "SoundCue Object Reference"))
  (bind _activesoundloop (`self.activeSoundLoop`))
  (if (`KismetSystemLibrary.IsValid` (`self.activeSoundLoop`))
    (`AudioComponent.Stop` _activesoundloop)
    (`ActorComponent.K2_DestroyComponent` _activesoundloop)
    (bind _returnvalue (`GameplayStatics.SpawnSound2D` sound 1.0 1.0 0.0 null))
    (set `self.activeSoundLoop` _returnvalue)
    (else
      (bind _returnvalue_2 (`GameplayStatics.SpawnSound2D` sound 1.0 1.0 0.0 null))
      (set `self.activeSoundLoop` _returnvalue_2))))

(event `ClientEvent RunFinished`
  (params (victoryData :type "Array of /Game/CampusClash/Core/Struct/STR_PlayerVictoryInfo Structure") (resultText :type String))
  (bind _returnvalue (`|CreateWidget` "/Game/CampusClash/Core/UI/MiniGames/VictoryScreen/WBP_VictoryScreen.WBP_VictoryScreen_C" (`GameplayStatics.GetPlayerController` 0) (`KismetTextLibrary.Conv_StringToText` resultText) victoryData))
  (`UserWidget.AddToViewport` _returnvalue 0))

(event `self.ReceiveUnpossessed`
  (params (OldController :type "Controller Object Reference"))
  (`self.OnDc` self))

(fn `DestroyWidget`
  (params (widget :type "Widget Object Reference"))
  (if (`KismetSystemLibrary.IsValid` widget)
    (`Widget.RemoveFromParent` widget)))

(fn `InitCountdownWidget`
  (bind _asbp_player_controller (cast `/Game/CampusClash/Core/Controllers/BP_PlayerController` (`GameplayStatics.GetPlayerController` 0)))
  (bind _returnvalue (`|CreateWidget` "/Game/CampusClash/Core/UI/MiniGames/FindYourWay/WBP_FYW_Countdown.WBP_FYW_Countdown_C" _asbp_player_controller))
  (bind _output_get (set `self.countdownWidget` _returnvalue))
  (`UserWidget.AddToViewport` _output_get 0))

(fn `InitEndWidget`
  (params (victoryData :type "Array of /Game/CampusClash/Core/Struct/STR_PlayerVictoryInfo Structure") (resultText :type Text))
  (locals (playerInfos :type "Array of /Game/CampusClash/Core/Struct/STR_PlayerVictoryInfo Structure"))
  (bind _returnvalue (`|CreateWidget` "/Game/CampusClash/Core/UI/MiniGames/VictoryScreen/WBP_VictoryScreen.WBP_VictoryScreen_C" (`GameplayStatics.GetPlayerController` 0) resultText victoryData))
  (bind _output_get (set `self.endWidget` _returnvalue))
  (`UserWidget.AddToViewport` _output_get 0))

(fn `UserConstructionScript`
  (`parent.UserConstructionScript`))