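; BP_rotationpumper is a bumper actor in the Mikrowellenspiel prototype that knocks away whatever overlaps its three bounce zones.
; All zones share one response: BP_ThirdPersonCharacter gets LaunchCharacter, anything else gets an impulse on the overlapping component.
; Both vectors are the actor's world-space bounds origin scaled by separate strength variables, so direction follows the bumper's position, not the contact side.
; The graph contains no rotation logic.
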(event `self.bounce zone.OnComponentBeginOverlap`
  (params (OverlappedComponent :type "PrimitiveComponent Object Reference") (OtherActor :type "Actor Object Reference") (OtherComp :type "PrimitiveComponent Object Reference") (OtherBodyIndex :type Integer) (bFromSweep :type Boolean) (SweepResult :type "HitResult Structure (by ref)"))
  (bind _origin (`self.GetActorBounds` true true))
  (bind _asbp_third_person_character (cast `/Game/StarterContent/ThirdPerson/Blueprints/BP_ThirdPersonCharacter` OtherActor)
    (:`then`
      (`Character.LaunchCharacter` _asbp_third_person_character (* _origin (`self.Character Bounce Strenght`)) false false :!label _label)
      (`Character.LaunchCharacter` (stale `self.bounce zone1.OnComponentBeginOverlap` _asbp_third_person_character) (* _origin (`self.Character Bounce Strenght`)) false false)
      (`Character.LaunchCharacter` (stale `self.bounce zone2.OnComponentBeginOverlap` _asbp_third_person_character) (* _origin (`self.Character Bounce Strenght`)) false false))
    (:`CastFailed`
      (`PrimitiveComponent.AddImpulse` (stale `self.bounce zone2.OnComponentBeginOverlap` OtherComp) (* _origin (`self.Physic Bounce Strenght_0`)) "None" false :!label _label_2)
      (`PrimitiveComponent.AddImpulse` (stale `self.bounce zone1.OnComponentBeginOverlap` OtherComp) (* _origin (`self.Physic Bounce Strenght_0`)) "None" false)
      (`PrimitiveComponent.AddImpulse` OtherComp (* _origin (`self.Physic Bounce Strenght_0`)) "None" false))))

(event `self.bounce zone1.OnComponentBeginOverlap`
  (params (OverlappedComponent :type "PrimitiveComponent Object Reference") (OtherActor :type "Actor Object Reference") (OtherComp :type "PrimitiveComponent Object Reference") (OtherBodyIndex :type Integer) (bFromSweep :type Boolean) (SweepResult :type "HitResult Structure (by ref)"))
  (bind _asbp_third_person_character (cast `/Game/StarterContent/ThirdPerson/Blueprints/BP_ThirdPersonCharacter` OtherActor)
    (:`then`
      (goto _label))
    (:`CastFailed`
      (goto _label_2))))

(event `self.bounce zone2.OnComponentBeginOverlap`
  (params (OverlappedComponent :type "PrimitiveComponent Object Reference") (OtherActor :type "Actor Object Reference") (OtherComp :type "PrimitiveComponent Object Reference") (OtherBodyIndex :type Integer) (bFromSweep :type Boolean) (SweepResult :type "HitResult Structure (by ref)"))
  (bind _asbp_third_person_character (cast `/Game/StarterContent/ThirdPerson/Blueprints/BP_ThirdPersonCharacter` OtherActor)
    (:`then`
      (goto _label))
    (:`CastFailed`
      (goto _label_2))))

(fn `UserConstructionScript`)