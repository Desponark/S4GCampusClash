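; BP_MazeWall is a prototype maze wall that the player raises by clicking its placeholder area.
; On BeginPlay it enables click events on the first player controller, then hides the Wall component and disables its collision.
; Clicking the Wallarea component hides that area and shows the Wall with query and physics collision.
; The graph has no path to lower the wall again.
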(event `self.ReceiveBeginPlay`
  (set `PlayerController.bEnableClickEvents` true (`GameplayStatics.GetPlayerController` 0))
  (`SceneComponent.SetVisibility` (`self.wall`) false false)
  (`PrimitiveComponent.SetCollisionEnabled` (`self.wall`) "NoCollision"))

(event `self.wallarea.OnClicked`
  (params (TouchedComponent :type "PrimitiveComponent Object Reference") (ButtonPressed :type "Key Structure"))
  (`SceneComponent.SetVisibility` (`self.wallarea`) false false)
  (`SceneComponent.SetVisibility` (`self.wall`) true false)
  (`PrimitiveComponent.SetCollisionEnabled` (`self.wall`) "QueryAndPhysics"))

(fn `UserConstructionScript`)