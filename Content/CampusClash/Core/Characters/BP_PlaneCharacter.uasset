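; BP_PlaneCharacter is a player-controlled plane character that moves forward continuously.
; Enhanced Input look steers controller yaw and pitch, while move X adds roll and positive move Y adds thrust along the control rotation's forward vector.
; Tick constantly applies movement input along the capsule's forward vector, providing baseline propulsion.
; A mesh look-at rotation snippet is left unwired and never runs.
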(event `EnhancedInput|/Game/CampusClash/Core/Input/Actions/IA_Look`
  (params (ActionValue :type "Vector2D Structure") (ElapsedSeconds :type "Float (double-precision)") (TriggeredSeconds :type "Float (double-precision)") (InputAction :type "InputAction Object Reference" :default "/Game/CampusClash/Core/Input/Actions/IA_Look.IA_Look"))
  (:`Triggered`
    (`self.AddControllerYawInput` ActionValue_X)
    (`self.AddControllerPitchInput` ActionValue_Y)))

(event `EnhancedInput|/Game/CampusClash/Core/Input/Actions/IA_Move`
  (params (ActionValue :type "Vector2D Structure") (ElapsedSeconds :type "Float (double-precision)") (TriggeredSeconds :type "Float (double-precision)") (InputAction :type "InputAction Object Reference" :default "/Game/CampusClash/Core/Input/Actions/IA_Move.IA_Move"))
  (bind (_returnvalue_roll _returnvalue_pitch _returnvalue_yaw) (`KismetMathLibrary.BreakRotator` (`self.GetControlRotation`)))
  (:`Triggered`
    (`self.AddControllerRollInput` ActionValue_X)
    (if (> ActionValue_Y 0.0)
      (`self.AddMovementInput` (`KismetMathLibrary.GetForwardVector` (`KismetMathLibrary.MakeRotator` _returnvalue_roll _returnvalue_pitch _returnvalue_yaw)) ActionValue_Y))))

(event `self.ReceiveTick`
  (params (DeltaSeconds :type "Float (single-precision)"))
  (`self.AddMovementInput` (`SceneComponent.GetForwardVector` (`self.CapsuleComponent`)) 0.8))

(fn `UserConstructionScript`)