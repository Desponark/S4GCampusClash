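; Placeable two-player quiz Tic-Tac-Toe station where players claim fields by answering category questions correctly.
; Joining players possess the station's player pawns, a random one starts, and turns alternate through client input and turn-info events.
; Multicasts update the shared 3D board widget; wrong answers re-roll the field's category.
; A winning line awards GameState points, and win or cancel returns players to their characters.
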(event `self.ReceiveBeginPlay`
  (`self.Initialize`))

(event `StartGame`
  (bind _player (`self.RandomStartPlayer`))
  (`self.SetActivePlayer` _player)
  (`self.UpdateTurnInfo`)
  (`self.SetCategories`)
  (`KismetSystemLibrary.Delay` 0.5)
  (`self.MultiCast ShowCategories`)
  (`/Game/CampusClash/Placeables/TicTacToeGame/BP_TicTacToe_Player.ClientEvent PlaySoundLooped` (`self.player1`) (`BlueprintMapLibrary.Map_Find` (`self.soundList`) "Background"))
  (`/Game/CampusClash/Placeables/TicTacToeGame/BP_TicTacToe_Player.ClientEvent PlaySoundLooped` (`self.player2`) (`BlueprintMapLibrary.Map_Find` (`self.soundList`) "Background"))
  (set `self.isInputLocked` false)
  (set `self.isGameOngoing` true)
  (set `self.isPlayerWaiting` false))

(event `EndGame`
  (params (winner :type "/Game/CampusClash/Placeables/TicTacToeGame/BP_TicTacToe_Player Object Reference"))
  (`KismetSystemLibrary.Delay` 1.5)
  (`self.Multicast EndGame`)
  (`self.UpdatePoints` winner)
  (`self.SetEndScreen` false winner)
  (`self.PlayerExit` (`self.player1`))
  (`self.PlayerExit` (`self.player2`))
  (`self.Reset`))

(event `CancelGame`
  (`self.SetEndScreen` true)
  (`self.PlayerExit` (`self.player1`))
  (`self.PlayerExit` (`self.player2`))
  (`self.Reset`))

(event `EndRound`
  (`self.SwitchActivePlayer`)
  (`self.UpdateTurnInfo`)
  (`self.Multicast EndRound`))

(event `self.OnInteraction`
  (params (InteractingPlayer :type "Actor Object Reference"))
  (if (not (`self.isGameOngoing`))
    (bind _aspawn (cast `Pawn` InteractingPlayer))
    (bind _asbp_player_controller (cast `/Game/CampusClash/Core/Controllers/BP_PlayerController` (`Pawn.GetController` _aspawn)))
    (`self.PlayerJoin` _asbp_player_controller)))

(event `PlayerJoin`
  (params (player :type "/Game/CampusClash/Core/Controllers/BP_PlayerController Object Reference"))
  (if (`self.isPlayerWaiting`)
    (bind _asbp_third_person_character (cast `/Game/StarterContent/ThirdPerson/Blueprints/BP_ThirdPersonCharacter` (`Controller.K2_GetPawn` player)))
    (set `self.mainCharacter2` _asbp_third_person_character)
    (`self.SetPlayerReady` player (`self.player2`))
    (`self.StartGame`)
    (else
      (`self.Reset`)
      (bind _asbp_third_person_character_2 (cast `/Game/StarterContent/ThirdPerson/Blueprints/BP_ThirdPersonCharacter` (`Controller.K2_GetPawn` player)))
      (set `self.mainCharacter1` _asbp_third_person_character_2)
      (set `self.isPlayerWaiting` true)
      (`self.SetPlayerReady` player (`self.player1`))
      (`/Game/CampusClash/Placeables/TicTacToeGame/BP_TicTacToe_Player.ClientEvent PlaySoundLooped` (`self.player1`) (`BlueprintMapLibrary.Map_Find` (`self.soundList`) "WaitForOpponent")))))

(event `test round switch`
  (params (p :type "/Game/CampusClash/Core/Controllers/BP_PlayerController Object Reference"))
  (`self.EndRound`))

(event `PlayerExit`
  (params (player :type "/Game/CampusClash/Placeables/TicTacToeGame/BP_TicTacToe_Player Object Reference"))
  (bind _maincharacter1 (`self.mainCharacter1`))
  (bind _maincharacter2 (`self.mainCharacter2`))
  (`/Game/CampusClash/Placeables/TicTacToeGame/BP_TicTacToe_Player.ClientEvent Exit` player)
  (bind _asbp_player_controller (cast `/Game/CampusClash/Core/Controllers/BP_PlayerController` (`Pawn.GetController` player)))
  (`Controller.UnPossess` _asbp_player_controller)
  (if (== (`self.player1`) player)
    (`Controller.Possess` _asbp_player_controller _maincharacter1)
    (`CharacterMovementComponent.SetMovementMode` (`Character.CharacterMovement` _maincharacter1) "MOVE_Walking" 0)
    (else
      (`Controller.Possess` _asbp_player_controller _maincharacter2)
      (`CharacterMovementComponent.SetMovementMode` (`Character.CharacterMovement` _maincharacter2) "MOVE_Walking" 0))))

(event `PlayerClickExit`
  (params (player :type "/Game/CampusClash/Placeables/TicTacToeGame/BP_TicTacToe_Player Object Reference"))
  (if (`self.isGameOngoing`)
    (`self.CancelGame`)
    (else
      (`self.PlayerExit` (`self.player1`))
      (`self.Reset`))))

(event `TryCardZoom`
  (params (card :type "/Game/CampusClash/Placeables/MemoryGame/BP_Card Object Reference") (player :type "/Game/CampusClash/Placeables/MemoryGame/BP_MemoryPlayer Object Reference"))
  (if (== player (`self.activePlayer`))
    (if (`self.cardsSelected`)
      (`KismetSystemLibrary.PrintString` "error: cards already selected")
      (else
        (set `/Game/CampusClash/Placeables/MemoryGame/BP_Card.hoveredOver` true card)
        (`KismetSystemLibrary.PrintString` (`KismetStringLibrary.Conv_BoolToString` (`/Game/CampusClash/Placeables/MemoryGame/BP_Card.hoveredOver` card)))))
    (else
      (`KismetSystemLibrary.PrintString` "error: controller not local"))))

(event `CardUnzoom`
  (params (card :type "/Game/CampusClash/Placeables/MemoryGame/BP_Card Object Reference") (player :type "/Game/CampusClash/Placeables/MemoryGame/BP_MemoryPlayer Object Reference"))
  (if (== player (`self.activePlayer`))
    (set `/Game/CampusClash/Placeables/MemoryGame/BP_Card.hoveredOver` false card)))

(event `ButtonClicked`
  (params (index :type Integer))
  (`self.ProcessClickedField` index))

(event `AnswerSelected`
  (params (isCorrect :type Boolean))
  (bind _fielddata (`self.fieldData`))
  (bind _activefieldindex (`self.activeFieldIndex`))
  (bind _output_category (break `/Game/CampusClash/Core/Struct/STR_TicTacToe_FieldData` (`|GetArrayItem` _fielddata _activefieldindex)))
  (if isCorrect
    (`KismetSystemLibrary.PrintString` "correct answer" true true (struct :`G` 0.66 :`B` 1.0 :`A` 1.0) 6.0)
    (`KismetArrayLibrary.Array_Set` _fielddata _activefieldindex (make `/Game/CampusClash/Core/Struct/STR_TicTacToe_FieldData` _output_category (`self.activePlayer`)))
    (if (== (`self.activePlayer`) (`self.player1`))
      (`self.MultiCast ShowFieldWinner` (`self.activeFieldIndex`) (`self.imageP1`))
      (bind _iswinner (`self.CheckForWin`))
      (if _iswinner
        (`self.EndGame` (`self.activePlayer`))
        (else
          (`self.EndRound`)))
      (else
        (`self.MultiCast ShowFieldWinner` (`self.activeFieldIndex`) (`self.imageP2`))
        (bind _iswinner_2 (`self.CheckForWin`))
        (if _iswinner_2
          (`self.EndGame` (`self.activePlayer`))
          (else
            (`self.EndRound`)))))
    (else
      (`KismetSystemLibrary.PrintString` "correct answer" true true (struct :`G` 0.66 :`B` 1.0 :`A` 1.0) 6.0)
      (bind _category (`self.GetCategory`))
      (`KismetArrayLibrary.Array_Set` (`self.fieldData`) (`self.activeFieldIndex`) (make `/Game/CampusClash/Core/Struct/STR_TicTacToe_FieldData` _category null))
      (`self.EndRound`))))

(event `MultiCast ShowCategories`
  (`self.ShowCategories`))

(event `Multicast ShowQuestion`
  (params (question :type "/Game/CampusClash/Core/Struct/STR_TicTacToe_Question Structure") (fieldIndex :type Integer))
  (bind _aswbp_quic_quac_quoc_3d (cast `/Game/CampusClash/Core/UI/MiniGames/TicTacToe/WBP_QuicQuacQuoc_3D` (`WidgetComponent.GetWidget` (`self.3DWidget`))))
  (`KismetSystemLibrary.PrintString` "show question game")
  (`/Game/CampusClash/Core/UI/MiniGames/TicTacToe/WBP_QuicQuacQuoc_3D.ShowQuestion` _aswbp_quic_quac_quoc_3d question fieldIndex))

(event `MultiCast ShowFieldWinner`
  (params (fieldIndex :type Integer) (image :type "Texture2D Object Reference"))
  (bind _aswbp_quic_quac_quoc_3d (cast `/Game/CampusClash/Core/UI/MiniGames/TicTacToe/WBP_QuicQuacQuoc_3D` (`WidgetComponent.GetWidget` (`self.3DWidget`))))
  (`/Game/CampusClash/Core/UI/MiniGames/TicTacToe/WBP_QuicQuacQuoc_3D.SetFieldWinner` _aswbp_quic_quac_quoc_3d image fieldIndex))

(event `Multicast EndRound`
  (bind _aswbp_quic_quac_quoc_3d (cast `/Game/CampusClash/Core/UI/MiniGames/TicTacToe/WBP_QuicQuacQuoc_3D` (`WidgetComponent.GetWidget` (`self.3DWidget`))))
  (`/Game/CampusClash/Core/UI/MiniGames/TicTacToe/WBP_QuicQuacQuoc_3D.TurnEnd` _aswbp_quic_quac_quoc_3d (`self.activeFieldIndex`)))

(event `Multicast EndGame`
  (bind _aswbp_quic_quac_quoc_3d (cast `/Game/CampusClash/Core/UI/MiniGames/TicTacToe/WBP_QuicQuacQuoc_3D` (`WidgetComponent.GetWidget` (`self.3DWidget`))))
  (`/Game/CampusClash/Core/UI/MiniGames/TicTacToe/WBP_QuicQuacQuoc_3D.Reset` _aswbp_quic_quac_quoc_3d))

(fn `CheckForWin`
  (returns (isWinner :type Boolean))
  (bind _iswinner (`self.CheckLineForWin` 0 1 2))
  (if _iswinner
    (return true)
    (else
      (bind _iswinner_2 (`self.CheckLineForWin` 3 4 5))
      (if _iswinner_2
        (return true)
        (else
          (bind _iswinner_3 (`self.CheckLineForWin` 6 7 8))
          (if _iswinner_3
            (return true)
            (else
              (bind _iswinner_4 (`self.CheckLineForWin` 0 3 6))
              (if _iswinner_4
                (return true)
                (else
                  (bind _iswinner_5 (`self.CheckLineForWin` 1 4 7))
                  (if _iswinner_5
                    (return true)
                    (else
                      (bind _iswinner_6 (`self.CheckLineForWin` 2 5 8))
                      (if _iswinner_6
                        (return true)
                        (else
                          (bind _iswinner_7 (`self.CheckLineForWin` 0 4 8))
                          (if _iswinner_7
                            (return true)
                            (else
                              (`self.CheckLineForWin` 2 4 6)
                              (return false))))))))))))))))

(fn `CheckLineForWin`
  (params (index1 :type Integer) (index2 :type Integer) (index3 :type Integer))
  (returns (isWinner :type Boolean))
  (bind (_output_category _output_owningplayer) (break `/Game/CampusClash/Core/Struct/STR_TicTacToe_FieldData` (`|GetArrayItem` (`self.fieldData`) index1)))
  (if (== (`self.activePlayer`) _output_owningplayer)
    (if (== (`self.activePlayer`) (`.owningPlayer_9_A95AAED645E1A4B813D41DAEE6359C07` (break `/Game/CampusClash/Core/Struct/STR_TicTacToe_FieldData` (`|GetArrayItem` (`self.fieldData`) index2))))
      (if (== (`self.activePlayer`) (`.owningPlayer_9_A95AAED645E1A4B813D41DAEE6359C07` (break `/Game/CampusClash/Core/Struct/STR_TicTacToe_FieldData` (`|GetArrayItem` (`self.fieldData`) index3))))
        (return true)
        (else
          (return false)))
      (else
        (return false)))
    (else
      (return false))))

(fn `DestroyCards`
  (for _array_element _
    (if (`KismetSystemLibrary.IsValid` _array_element)
      (`self.K2_DestroyActor` _array_element))))

(fn `DestroyJoinWidget`
  (`Widget.RemoveFromParent` (`self.localJoinWidget`)))

(fn `DetermineWinner`
  (returns (winner :type "/Game/CampusClash/Placeables/TicTacToeGame/BP_TicTacToe_Player Object Reference"))
  (return null))

(fn `GetActorUnderMouse`
  (returns (hitActor :type "Actor Object Reference"))
  (bind _returnvalue (`GameplayStatics.GetPlayerController` 0))
  (if (`KismetSystemLibrary.IsValid` _returnvalue)
    (return (`.HitActor` (`GameplayStatics.BreakHitResult` (`PlayerController.GetHitResultUnderCursorByChannel` _returnvalue "TraceTypeQuery2" true))))))

(fn `GetCategory`
  (returns (category :type "/Game/CampusClash/Core/Struct/STR_TicTacToe_Category Structure"))
  (locals (result :type "/Game/CampusClash/Core/Struct/STR_TicTacToe_Category Structure") (randomIndex :type Integer))
  (bind _output_get (set `local.randomIndex` (`KismetMathLibrary.RandomInteger` (`KismetArrayLibrary.Array_Length` (`.Value_3_196A86764937B148F36CFA86DF4C4915` (break `/Game/CampusClash/Core/Struct/STR_TicTacToe_Categories` (`self.categories`)))))))
  (bind _output_get_2 (set `local.result` (`|GetArrayItem` (`.Value_3_196A86764937B148F36CFA86DF4C4915` (break `/Game/CampusClash/Core/Struct/STR_TicTacToe_Categories` (`self.categories`))) _output_get)))
  (`KismetArrayLibrary.Array_Remove` (`.Value_3_196A86764937B148F36CFA86DF4C4915` (break `/Game/CampusClash/Core/Struct/STR_TicTacToe_Categories` (`self.categories`))) _output_get)
  (return _output_get_2))

(fn `GetNeighbours`
  (params (x :type Integer) (y :type Integer))
  (returns (topNeighbourId :type Integer) (botNeighbourId :type Integer) (leftNeighbourId :type Integer) (rightNeighbourId :type Integer))
  (locals (top :type Integer) (bot :type Integer) (left :type Integer) (right :type Integer))
  (bind _returnvalue (+ 0 -1))
  (bind _returnvalue_2 (+ x 1))
  (bind _returnvalue_3 (+ (`local.x`) -1))
  (bind _returnvalue_4 (+ (`local.y`) 1))
  (if (< _returnvalue_2 3)
    (set `local.right` (+ _returnvalue_2 (* y 3)))
    (else
      (set `local.right` -1)))
  (if (> _returnvalue_3 -1)
    (set `local.left` (+ _returnvalue_3 (* (`local.y`) 3)))
    (else
      (set `local.left` 0)))
  (if (< _returnvalue_4 3)
    (set `local.top` (+ (`local.x`) (* _returnvalue_4 3)))
    (else
      (set `local.top` 0)))
  (if (> _returnvalue -1)
    (set `local.bot` (+ (`local.x`) (* _returnvalue 3)))
    (else
      (set `local.bot` 0)))
  (return (`local.top`) (`local.bot`) (`local.left`) (`local.right`)))

(fn `InitGameWidget`
  (params (player :type "/Game/CampusClash/Placeables/TicTacToeGame/BP_TicTacToe_Player Object Reference"))
  (`/Game/CampusClash/Core/UI/MiniGames/TicTacToe/WBP_QuicQuacQuoc_3D.Initialize` (`self.gameWidget`) self))

(fn `Initialize`
  (bind _aswbp_quic_quac_quoc_3d (cast `/Game/CampusClash/Core/UI/MiniGames/TicTacToe/WBP_QuicQuacQuoc_3D` (`WidgetComponent.GetWidget` (`self.3DWidget`))))
  (bind _output_get (set `self.gameWidget` _aswbp_quic_quac_quoc_3d))
  (`/Game/CampusClash/Core/UI/MiniGames/TicTacToe/WBP_QuicQuacQuoc_3D.Initialize` _output_get self)
  (`/Game/CampusClash/Core/UI/MiniGames/TicTacToe/WBP_QuicQuacQuoc_3D.Reset` _output_get)
  (set `self.imageP1` "/Game/CampusClash/Art/Assets/TicTacToe/Icon_Controller.Icon_Controller")
  (set `self.imageP2` "/Game/CampusClash/Art/Assets/TicTacToe/Icon_KeyboardMouse.Icon_KeyboardMouse"))

(fn `InteractionPrompt`
  (returns (IsEnabled :type Boolean) (Text :type Text))
  (if (`self.isGameOngoing`)
    (return true "Game has already started")
    (else
      (return true " Play Tic Tac Toe"))))

(fn `OnRep_fieldData`)

(fn `PlayPairResultSound`
  (params (player1Successful :type Boolean))
  (if player1Successful
    (`/Game/CampusClash/Placeables/TicTacToeGame/BP_TicTacToe_Player.ClientEvent PlaySound` (`self.player1`) (`BlueprintMapLibrary.Map_Find` (`self.soundList`) "CardsMatch"))
    (`/Game/CampusClash/Placeables/TicTacToeGame/BP_TicTacToe_Player.ClientEvent PlaySound` (`self.player2`) (`BlueprintMapLibrary.Map_Find` (`self.soundList`) "CardsMismatch"))
    (else
      (`/Game/CampusClash/Placeables/TicTacToeGame/BP_TicTacToe_Player.ClientEvent PlaySound` (`self.player2`) (`BlueprintMapLibrary.Map_Find` (`self.soundList`) "CardsMatch"))
      (`/Game/CampusClash/Placeables/TicTacToeGame/BP_TicTacToe_Player.ClientEvent PlaySound` (`self.player1`) (`BlueprintMapLibrary.Map_Find` (`self.soundList`) "CardsMismatch")))))

(fn `ProcessClickedField`
  (params (fieldIndex :type Integer))
  (locals (randomIndex :type Integer))
  (bind _output (`|GetArrayItem` (`self.fieldData`) fieldIndex))
  (bind _output_get (set `local.randomIndex` (`KismetMathLibrary.RandomInteger` (`KismetArrayLibrary.Array_Length` (`.Questions_6_DEA13AEA4AAD80ECE198F4AA55A6A84E` (break `/Game/CampusClash/Core/Struct/STR_TicTacToe_Category` (break `/Game/CampusClash/Core/Struct/STR_TicTacToe_FieldData` _output)))))))
  (`self.Multicast ShowQuestion` (`|GetArrayItem` (`.Questions_6_DEA13AEA4AAD80ECE198F4AA55A6A84E` (break `/Game/CampusClash/Core/Struct/STR_TicTacToe_Category` (break `/Game/CampusClash/Core/Struct/STR_TicTacToe_FieldData` _output))) _output_get) fieldIndex)
  (set `self.activeFieldIndex` fieldIndex)
  (`KismetArrayLibrary.Array_Remove` (`.Questions_6_DEA13AEA4AAD80ECE198F4AA55A6A84E` (break `/Game/CampusClash/Core/Struct/STR_TicTacToe_Category` (break `/Game/CampusClash/Core/Struct/STR_TicTacToe_FieldData` _output))) (`local.randomIndex`)))

(fn `RandomStartPlayer`
  (returns (player :type "/Game/CampusClash/Placeables/TicTacToeGame/BP_TicTacToe_Player Object Reference"))
  (if (> (`KismetMathLibrary.RandomFloat`) 0.5)
    (return (`self.player1`))
    (else
      (return (`self.player2`)))))

(fn `Reset`
  (set `self.isInputLocked` false)
  (`/Game/CampusClash/Placeables/TicTacToeGame/BP_TicTacToe_Player.Reset` (`self.player1`))
  (`/Game/CampusClash/Placeables/TicTacToeGame/BP_TicTacToe_Player.Reset` (`self.player2`))
  (set `self.activePlayer` null)
  (set `self.isPlayerWaiting` false)
  (set `self.isGameOngoing` false)
  (set `self.cardsSelected` false))

(fn `SetActivePlayer`
  (params (player :type "/Game/CampusClash/Placeables/TicTacToeGame/BP_TicTacToe_Player Object Reference"))
  (bind _output_get (set `self.activePlayer` player))
  (if (== _output_get (`self.player1`))
    (`/Game/CampusClash/Placeables/TicTacToeGame/BP_TicTacToe_Player.ClientEvent ActivateInput` (`self.player1`) self)
    (`/Game/CampusClash/Placeables/TicTacToeGame/BP_TicTacToe_Player.ClientEvent DeactivateInput` (`self.player2`) self)
    (else
      (`/Game/CampusClash/Placeables/TicTacToeGame/BP_TicTacToe_Player.ClientEvent DeactivateInput` (`self.player1`) self)
      (`/Game/CampusClash/Placeables/TicTacToeGame/BP_TicTacToe_Player.ClientEvent ActivateInput` (`self.player2`) self))))

(fn `SetCategories`
  (locals (tempFieldData :type "Array of /Game/CampusClash/Core/Struct/STR_TicTacToe_FieldData Structure") (randomIndex :type Integer))
  (for _ (range 9)
    (bind _category (`self.GetCategory`))
    (`KismetArrayLibrary.Array_Add` (`local.tempFieldData`) (make `/Game/CampusClash/Core/Struct/STR_TicTacToe_FieldData` _category null)))
  (set `self.fieldData` (`local.tempFieldData`)))

(fn `SetEndScreen`
  (params (isGameCancelled :type Boolean) (winner :type "/Game/CampusClash/Placeables/TicTacToeGame/BP_TicTacToe_Player Object Reference"))
  (locals (controllerP1 :type "/Game/CampusClash/Core/Controllers/BP_PlayerController Object Reference") (controllerP2 :type "/Game/CampusClash/Core/Controllers/BP_PlayerController Object Reference"))
  (if isGameCancelled
    _
    (elif (`KismetSystemLibrary.IsValid` winner)
      (if (== winner (`self.player1`))
        (`/Game/CampusClash/Placeables/TicTacToeGame/BP_TicTacToe_Player.ClientEvent InitResultWidget` (`self.player1`) "Winner")
        (`/Game/CampusClash/Placeables/TicTacToeGame/BP_TicTacToe_Player.ClientEvent InitResultWidget` (`self.player2`) "Loser")
        (else
          (`/Game/CampusClash/Placeables/TicTacToeGame/BP_TicTacToe_Player.ClientEvent InitResultWidget` (`self.player1`) "Loser")
          (`/Game/CampusClash/Placeables/TicTacToeGame/BP_TicTacToe_Player.ClientEvent InitResultWidget` (`self.player2`) "Winner"))))))

(fn `SetInteractability`
  (params (isInteractable :type Boolean))
  (bind _aswbp_quic_quac_quoc_3d (cast `/Game/CampusClash/Core/UI/MiniGames/TicTacToe/WBP_QuicQuacQuoc_3D` (`WidgetComponent.GetWidget` (`self.3DWidget`))))
  (`/Game/CampusClash/Core/UI/MiniGames/TicTacToe/WBP_QuicQuacQuoc_3D.SetInteractabilityFields` _aswbp_quic_quac_quoc_3d isInteractable))

(fn `SetNeighbourFields`
  (locals (index :type Integer)))

(fn `SetPlayerReady`
  (params (controller :type "/Game/CampusClash/Core/Controllers/BP_PlayerController Object Reference") (player :type "/Game/CampusClash/Placeables/TicTacToeGame/BP_TicTacToe_Player Object Reference"))
  (bind _asbp_third_person_character (cast `/Game/StarterContent/ThirdPerson/Blueprints/BP_ThirdPersonCharacter` (`Controller.K2_GetPawn` controller)))
  (`MovementComponent.StopMovementImmediately` (`Character.CharacterMovement` _asbp_third_person_character))
  (`Controller.Possess` controller player)
  (`/Game/CampusClash/Placeables/TicTacToeGame/BP_TicTacToe_Player.Initialize` player self)
  (`/Game/CampusClash/Placeables/TicTacToeGame/BP_TicTacToe_Player.ClientEvent InitPlayerWidget` player)
  (`/Game/CampusClash/Placeables/TicTacToeGame/BP_TicTacToe_Player.ClientEvent UpdateTurnInfo` player "Waiting For Opponent...")
  (add `/Game/CampusClash/Placeables/TicTacToeGame/BP_TicTacToe_Player.OnClickExit` player (`|CreateDelegate` :!event `PlayerClickExit`))
  (add `/Game/CampusClash/Placeables/TicTacToeGame/BP_TicTacToe_Player.OnClickField` player (`|CreateDelegate` :!event `ButtonClicked`))
  (`/Game/CampusClash/Placeables/TicTacToeGame/BP_TicTacToe_Player.ClientEvent DeactivateInput` player self)
  (bind _asbp_player_controller (cast `/Game/CampusClash/Core/Controllers/BP_PlayerController` (`Pawn.GetController` player)))
  (add `/Game/CampusClash/Core/Controllers/BP_PlayerController.OnCPressed` _asbp_player_controller (`|CreateDelegate` :!event `test round switch`)))

(fn `ShowCategories`
  (for _index (range 9)
    (bind _aswbp_quic_quac_quoc_3d (cast `/Game/CampusClash/Core/UI/MiniGames/TicTacToe/WBP_QuicQuacQuoc_3D` (`WidgetComponent.GetWidget` (`self.3DWidget`))))
    (`TextBlock.SetText` (`|GetArrayItem` (`/Game/CampusClash/Core/UI/MiniGames/TicTacToe/WBP_QuicQuacQuoc_3D.texts` _aswbp_quic_quac_quoc_3d) _index) (`KismetTextLibrary.Conv_StringToText` (break `/Game/CampusClash/Core/Struct/STR_TicTacToe_Category` (break `/Game/CampusClash/Core/Struct/STR_TicTacToe_FieldData` (`|GetArrayItem` (`self.fieldData`) _index)))))))

(fn `SwitchActivePlayer`
  (locals (activePlayerWidget :type "Object Object Reference") (inactivePlayerWidget :type "Object Object Reference"))
  (if (== (`self.player1`) (`self.activePlayer`))
    (`self.SetActivePlayer` (`self.player2`))
    (else
      (`self.SetActivePlayer` (`self.player1`)))))

(fn `TryStopHoverCard`
  (bind _hoveredcard (`self.hoveredCard`))
  (if (`KismetSystemLibrary.IsValid` _hoveredcard)
    (if (`/Game/CampusClash/Placeables/MemoryGame/BP_Card.hoveredOver` _hoveredcard)
      (`/Game/CampusClash/Placeables/MemoryGame/BP_Card.StopHover` _hoveredcard)
      (set `self.hoveredCard` null))))

(fn `UpdatePoints`
  (params (winner :type "/Game/CampusClash/Placeables/TicTacToeGame/BP_TicTacToe_Player Object Reference"))
  (if (`KismetSystemLibrary.IsValid` winner)
    (bind _asbp_player_controller (cast `/Game/CampusClash/Core/Controllers/BP_PlayerController` (`Pawn.GetController` winner)))
    (bind _asbp_game_state (cast `/Game/CampusClash/Core/GameStates/BP_GameState` (`GameplayStatics.GetGameState`)))
    (`/Game/CampusClash/Core/GameStates/BP_GameState.AddPoints` _asbp_game_state (`self.pointsForWin`) _asbp_player_controller)))

(fn `UpdateTurnInfo`
  (if (== (`self.player1`) (`self.activePlayer`))
    (`/Game/CampusClash/Placeables/TicTacToeGame/BP_TicTacToe_Player.ClientEvent UpdateTurnInfo` (`self.player1`) "Your turn")
    (`/Game/CampusClash/Placeables/TicTacToeGame/BP_TicTacToe_Player.ClientEvent UpdateTurnInfo` (`self.player2`) "OpponentsTurn")
    (else
      (`/Game/CampusClash/Placeables/TicTacToeGame/BP_TicTacToe_Player.ClientEvent UpdateTurnInfo` (`self.player1`) "OpponentsTurn")
      (`/Game/CampusClash/Placeables/TicTacToeGame/BP_TicTacToe_Player.ClientEvent UpdateTurnInfo` (`self.player2`) "YourTurn"))))

(fn `UserConstructionScript`)