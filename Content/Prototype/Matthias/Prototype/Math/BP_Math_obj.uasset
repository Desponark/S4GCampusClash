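; BP_Math_obj is a prototype math-level object, one of a pair of rotating cubes that must both stop to finish the level.
; When an overlap with its Box ends, delayed steps lower the RotatingMovement rate to zero and clear IsTurning.
; If the referenced OtherCube has also stopped, it shows the UI_Pointsreached widget, then opens the Campus level after a short delay.
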(event `self.Box.OnComponentEndOverlap`
  (params (OverlappedComponent :type "PrimitiveComponent Object Reference") (OtherActor :type "Actor Object Reference") (OtherComp :type "PrimitiveComponent Object Reference") (OtherBodyIndex :type Integer))
  (set `RotatingMovementComponent.RotationRate` (struct :`Yaw` 200.0) (`self.RotatingMovement`))
  (`KismetSystemLibrary.Delay` 1.0)
  (set `RotatingMovementComponent.RotationRate` (struct :`Yaw` 130.0) (`self.RotatingMovement`))
  (`KismetSystemLibrary.Delay` 1.0)
  (set `RotatingMovementComponent.RotationRate` (struct :`Yaw` 60.0) (`self.RotatingMovement`))
  (`KismetSystemLibrary.Delay` 1.0)
  (set `RotatingMovementComponent.RotationRate` (struct) (`self.RotatingMovement`))
  (set `self.isTurning` false)
  (if (not (`/Game/Prototype/Matthias/Prototype/Math/BP_Math_obj.isTurning` (`self.otherCube`)))
    (bind _returnvalue (`|CreateWidget` "/Game/Prototype/Matthias/Prototype/Math/UI/UI_Pointsreached.UI_Pointsreached_C"))
    (`UserWidget.AddToPlayerScreen` _returnvalue 0)
    (`KismetSystemLibrary.Delay` 3.0)
    (`GameplayStatics.OpenLevelBySoftObjectPtr` "/Game/CampusClash/Maps/Campus.Campus")))

(fn `UserConstructionScript`)